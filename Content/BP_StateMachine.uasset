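; BP_StateMachine is a state machine that switches between idle-walk-run, targeting and aiming states and delegates movement input to the active one.
; On BeginPlay it constructs one object per state and keeps each for reuse.
; SetState selects the current state from the requested value and calls its EnterState with the passed argument, with no exit call on the previous state.
; Move forwards input to the current state with X and Y swapped.
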(event `self.ReceiveBeginPlay`
  (`self.ConstructBeginPlay`))

(fn `ConstructBeginPlay`
  (bind _returnvalue (`|GenericCreateObject` "/Script/Lamp.BaseState"))
  (set `self.BaseState` _returnvalue)
  (bind _returnvalue_2 (`|GenericCreateObject` "/Script/Lamp.TargettingState"))
  (set `self.TargetingState` _returnvalue_2)
  (bind _returnvalue_3 (`|GenericCreateObject` "/Script/Lamp.AimingState"))
  (set `self.AimingState` _returnvalue_3))

(fn `Move`
  (params (InputX :type "Float (double-precision)") (`Input Y` :type "Float (double-precision)"))
  (`BaseState.Move` (`self.CurrentState`) `Input Y` InputX))

(fn `SetState`
  (params (NewParam :type "ENUM_States Enum" :default "IdleWalkRun") (NewParam1 :type "Map of String to Object Object Reference"))
  (`|ExecutionSequence`
    (:`then_0`
      (switch `ENUM_States` NewParam
        (:`IdleWalkRun`
          (set `self.CurrentState` (`self.BaseState`)))
        (:`Targeting`
          (set `self.CurrentState` (`self.TargetingState`)))
        (:`Aiming`
          (set `self.CurrentState` (`self.AimingState`)))))
    (:`then_1`
      (`BaseState.EnterState` (`self.CurrentState`) NewParam1))))