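; Test controller that turns directional input from IA_Movement into a current attack direction.
; On BeginPlay it adds the IMC_MainCharacter Enhanced Input mapping context.
; While input is active, it sets CurrentAttackInput to a right swing, left swing or stab, with any horizontal input taking priority over vertical.
; Downward, zero, canceled or completed input sets it to Neutral; nothing here moves a character or performs attacks.
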(event `self.ReceiveBeginPlay`
  (`EnhancedInputSubsystemInterface.AddMappingContext` (subsystem `EnhancedInputLocalPlayerSubsystem`) "/Game/InputManager/IMC_MainCharacter.IMC_MainCharacter" 0 (struct)))

(event `EnhancedInput|/Game/InputManager/Inputs/IA_Movement`
  (params (ActionValue :type "Vector2D Structure") (ElapsedSeconds :type "Float (double-precision)") (TriggeredSeconds :type "Float (double-precision)") (InputAction :type "InputAction Object Reference" :default "/Game/InputManager/Inputs/IA_Movement.IA_Movement"))
  (bind _returnvalue (!= ActionValue_X 0.0))
  (:`Triggered`
    (if (or _returnvalue (!= ActionValue_Y 0.0)) :!label _label
      (if _returnvalue
        (if (>= ActionValue_X 0.0)
          (set `self.CurrentAttackInput` "RightSwing")
          (else
            (set `self.CurrentAttackInput` "LeftSwing")))
        (elif (>= ActionValue_Y 0.0)
          (set `self.CurrentAttackInput` "Stab")
          (else
            (set `self.CurrentAttackInput` "Neutral"))))
      (else
        (set `self.CurrentAttackInput` "Neutral" :!label _label_2))))
  (:`Started`
    (goto _label))
  (:`Ongoing`
    (goto _label))
  (:`Canceled`
    (goto _label_2))
  (:`Completed`
    (goto _label_2)))

(fn `UserConstructionScript`)